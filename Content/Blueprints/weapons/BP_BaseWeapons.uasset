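; Base weapon Blueprint providing hitscan firing, with empty Shoot and EndShoot events, presumably for child weapons to override.
; CreateShotTrace plays a muzzle explosion and multi-line-traces Pawn objects forward from ShotArrow over a given range, applying Damage to each hit.
; Each hit also calls SpawnHitParticles, which picks a surface or blood effect from the actor's first tag, defaulting to ceramic, and orients it relative to the shot.
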(event Custom|CreateShotTrace
  (params (Range :type Float%20%28double-precision%29))
  (bind _shotarrow (Variables|Default|GetShotArrow))
  (bind _returnvalue (Transformation|GetWorldLocation _shotarrow))
  (bind _returnvalue_2 (Transformation|GetWorldRotation _shotarrow))
  (Effects|SpawnEmitterAttached "/Game/GTCaliberAssets/Content/Realistic_Starter_VFX_Pack_Vol2/Particles/Explosion/P_Explosion_Big_A.P_Explosion_Big_A" _shotarrow "None" "0, 0, 0" "0, 0, 0" "0.300000,0.300000,0.300000")
  (bind (_outhits _returnvalue_3) (Class|KismetSystemLibrary|LineTraceMultiforObjects _returnvalue (+ _returnvalue (* (Math|Vector|GetForwardVector _returnvalue_2) Range)) (Utilities|Array|MakeArray "ObjectTypeQuery3") false 0 "None" true))
  (if _returnvalue_3
    (bind _array_element (Utilities|Array|ForEachLoopwithBreak _outhits)
      (:LoopBody
        (CallFunction|SpawnHitParticles (Utilities|Array|Get(acopy) (Variables|/Script/Engine.Actor|GetTags (.HitActor (Collision|BreakHitResult _array_element)))) (.Location (Collision|BreakHitResult _array_element)) _returnvalue_2)
        (Game|Damage|ApplyDamage (.HitActor (Collision|BreakHitResult _array_element)) (Variables|Default|GetDamage) 0 0)))))

(event Custom|Shoot)

(event Custom|EndShoot)

(event Custom|SpawnHitParticles
  (params (TagName :type Name) (Location :type Vector) (ArrowRotation :type Rotator))
  (bind (_roll _pitch _yaw) (Math|Rotator|BreakRotator ArrowRotation))
  (switch name TagName
    (:Default
      (Variables|Default|SetHit%20Particles "/Game/GTCaliberAssets/Content/Realistic_Starter_VFX_Pack_Vol2/Particles/Destruction/P_Destruction_Ceramic.P_Destruction_Ceramic"))
    (:Wood
      (Variables|Default|SetHit%20Particles "/Game/GTCaliberAssets/Content/Realistic_Starter_VFX_Pack_Vol2/Particles/Destruction/P_Destruction_Wood.P_Destruction_Wood"))
    (:Metal
      (Variables|Default|SetHit%20Particles "/Game/GTCaliberAssets/Content/Realistic_Starter_VFX_Pack_Vol2/Particles/Destruction/P_Destruction_Metal.P_Destruction_Metal"))
    (:Brick
      (Variables|Default|SetHit%20Particles "/Game/GTCaliberAssets/Content/Realistic_Starter_VFX_Pack_Vol2/Particles/Destruction/P_Destruction_Concrete.P_Destruction_Concrete"))
    (:Glass
      (Variables|Default|SetHit%20Particles "/Game/GTCaliberAssets/Content/Realistic_Starter_VFX_Pack_Vol2/Particles/Destruction/P_Destruction_Glass.P_Destruction_Glass"))
    (:Concrete
      (Variables|Default|SetHit%20Particles "/Game/GTCaliberAssets/Content/Realistic_Starter_VFX_Pack_Vol2/Particles/Destruction/P_Destruction_Concrete.P_Destruction_Concrete"))
    (:Building
      (Variables|Default|SetHit%20Particles "/Game/GTCaliberAssets/Content/Realistic_Starter_VFX_Pack_Vol2/Particles/Destruction/P_Destruction_Building_A.P_Destruction_Building_A"))
    (:Creature
      (Variables|Default|SetHit%20Particles "/Game/GTCaliberAssets/Content/Realistic_Starter_VFX_Pack_Vol2/Particles/Blood/P_Blood_Splat_Cone.P_Blood_Splat_Cone")))
  (Effects|SpawnEmitteratLocation (Variables|Default|GetHit%20Particles) Location (Math|Rotator|MakeRotator _roll (+ _pitch 9e+01) _yaw) "0.400000,0.400000,0.400000"))

(fn ConstructionScript)